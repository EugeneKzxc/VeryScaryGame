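; BP_AntizeVOIPComponent is a character component providing proximity and team voice chat with push-to-talk state, per-listener muting and bip sounds.
; It creates a VOIP talker attached to the capsule, then swaps normal, team or mute attenuation locally per listener.
; Team changes relay attenuation updates through the server to affected clients.
; CheckForVOIP scans interface actors, using distance and line traces to drive speaker icons, HUD list and talker effect sound.
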(event Custom|OnDeath
  (bind _playerlisrref (Variables|Spawn|GetPlayerLisrRef))
  (bind _hudref (Variables|Spawn|GetHUDRef))
  ;[1 1 1] Disable VoIP, remove widget and invalidate timer on death
  (CallFunction|ActivateDeactivateVOIP false)
  (Utilities|Time|ClearandInvalidateTimerbyHandle (Variables|Spawn|GetTimer_CheckForLoop))
  (Utilities|IsValid _hudref
    (:Is%20Valid
      (Widget|RemovefromParent _hudref))
    (:Is%20Not%20Valid
      _))
  (Utilities|IsValid _playerlisrref
    (:Is%20Valid
      (Widget|RemovefromParent _playerlisrref))))

(event Custom|CreateVOIP
  (bind _characterref (Variables|Spawn|GetCharacterRef))
  ;[1 1 1] Create VOIP
  (bind _charref (Utilities|GetCharRef :!label _label)
    (:Is%20Valid
      (Utilities|IsValid (Variables|/Script/Engine.Pawn|GetPlayerState _charref)
        (:Is%20Valid
          (bind _returnvalue (Class|VOIPTalker|CreateTalkerforPlayer (Variables|/Script/Engine.Pawn|GetPlayerState _charref)))
          (bind _output_get (Variables|Default|SetMyVoiceRef _returnvalue))
          (Class|VOIPTalker|RegisterwithPlayerState _output_get (Variables|/Script/Engine.Pawn|GetPlayerState _characterref))
          (Class|VOIPStatics|SetMicThreshold -2e+01)
          (Variables|/Script/Engine.VOIPTalker|SetSettings (Variables|Default|GetMyVoiceRef) (Utilities|Struct|MakeVoiceSettings (Variables|/Script/Engine.Character|GetCapsuleComponent _characterref) "/Game/AntizeVOIPSystem/Audio/SA_VOIPAttenuation.SA_VOIPAttenuation")))
        (:Is%20Not%20Valid
          (Utilities|FlowControl|Delay 0.2 :!label _label_2)
          (goto _label))))
    (:NotValid
      (goto _label_2))))

(event Custom|Server_PlayBipOnPlayer
  (params (Sound :type Sound%20Cue%20Object%20Reference))
  ;[1 1 1] Play sound on player
  (CallFunction|ClientPlayBip Sound))

(event Custom|Client_RefreshAttenuationOnTeam
  (params (InSameTeam? :type Boolean) (FromPlayerRef :type Character%20Object%20Reference))
  ;[1 1 1] Call RefreshAttenuationOnTeam on client (OnTeam)
  (bind _reference (Utilities|GetComponentbyActorRef FromPlayerRef)
    (:IsValid
      (CallFunction|LocalRefreshAttenuationonTeam _reference InSameTeam?))))

(event Custom|Server_SendSetAttenuationOnTeam
  (params (InSameTeam? :type Boolean) (ToPlayerRef :type Character%20Object%20Reference) (FromPlayerRef :type Character%20Object%20Reference))
  ;[1 1 1] Call RefreshAttenuationOnTeam on client (OnTeam)
  (Utilities|MyHasAuthority
    (:Server
      (bind _reference (Utilities|GetComponentbyActorRef ToPlayerRef)
        (:IsValid
          (CallFunction|CallSetAttenuationonTeam _reference false InSameTeam? ToPlayerRef FromPlayerRef))))))

(event Custom|Server_SetTeamID
  (params (TeamID :type Integer))
  ;[1 1 1] Steam TeamID
  (Utilities|MyHasAuthority
    (:Server
      (Variables|Traitement|SetTeamID TeamID))))

(event Custom|Local_RefreshAttenuationOnTeam
  (params (InSameTeam :type Boolean))
  (bind _myvoiceref (Variables|Default|GetMyVoiceRef))
  ;[1 1 1] (Locally) Refresh the player attenuation
  (Utilities|IsValid _myvoiceref
    (:Is%20Valid
      (Utilities|Struct|SetmembersinVoiceSettings (Variables|/Script/Engine.VOIPTalker|GetSettings _myvoiceref) (Traitement|GetAttenutation InSameTeam (Variables|Traitement|Local|GetIsMuted?))))))

(event Custom|SecureMute
  ;[1 1 1] Secure
  (Development|ExecuteConsoleCommand "ToggleSpeaking 0" 0)
  (Utilities|FlowControl|Delay 0.35)
  (if (Variables|Traitement|GetIsVOIPActivated?)
    (Development|ExecuteConsoleCommand "ToggleSpeaking 1" 0)))

(event Custom|ActivateDeactivateVOIP
  (params (Activated? :type Boolean))
  (bind _hudref (Variables|Spawn|GetHUDRef))
  ;[1 1 1] Activate/Deactivate VoIP
  (Development|ExecuteConsoleCommand (select Activated? "ToggleSpeaking 1" "ToggleSpeaking 0") 0)
  (CallFunction|ServerSetVOIPActivated Activated?)
  (Utilities|FlowControl|Sequence
    (:then_0
      (Utilities|IsValid _hudref
        (:Is%20Valid
          (Default|SetVOIPIconVisibility _hudref Activated?))))
    (:then_1
      ;;[1 1 1] Play bip sound and spam protection
      (Utilities|FlowControl|DoOnce false :!label _label
        (:Completed
          (Utilities|FlowControl|Sequence
            (:then_0
              (Traitement|Sound|OnBip))
            (:then_1
              (Utilities|FlowControl|Delay 0.25)
              (goto _label Reset))))))))

(event Custom|MuteTemplate
  (params (PlayerIndex :type Integer))
  ;[1 1 1] Mute the player only at the one who called "MuteTemplate"
  (bind _outactors (Actor|GetAllActorswithInterface "/Game/AntizeVOIPSystem/Blueprints/BP_VOIPInterface.BP_VOIPInterface_C"))
  (if (Utilities|Array|IsValidIndex _outactors PlayerIndex)
    (Utilities|GetIsLocallyControlled (Utilities|Array|Get(acopy) _outactors PlayerIndex)
      (:false
        (bind _reference (Utilities|GetComponentbyActorRef (Utilities|Array|Get(acopy) _outactors PlayerIndex))
          (:IsValid
            (CallFunction|LocalSetIsMuted _reference (not (Variables|BP_AntizeVOIPComponent_C|GetIsMuted? _reference)) (Traitement|GetIsinSameTeam (Variables|BP_AntizeVOIPComponent_C|GetTeamID _reference) (Variables|Traitement|GetTeamID)))))))))

(event Custom|OnTimer_CheckForVOIP
  ;[1 1 1] Loop check for VoIP icon visibility
  (Utilities|GetCharRef
    (:Is%20Valid
      (Traitement|CheckforVOIP))))

(event Custom|Server_SetVOIPActivated
  (params (VOIPActivated? :type Boolean))
  ;[1 1 1] (Server) Replicate VoIPActivated variable
  (Utilities|MyHasAuthority
    (:Server
      (Variables|Traitement|SetIsVOIPActivated? VOIPActivated?))))

(event Custom|CallOnRepTeamID
  ;[1 1 1] OnRep TeamID
  (Utilities|RefreshAttenuation))

(event Custom|CallJoinTeam
  (params (NewTeamID :type Integer))
  ;[1 1 1] Join team
  (Traitement|OnJoinTeam NewTeamID))

(event Custom|Local_SetVisibilityVOIPIcon
  (params (Visible? :type Boolean))
  ;[1 1 1] (Locally) Set WidgetVoice visibility
  (if (Math|Boolean|NotEqual(Boolean) Visible? (Variables|Traitement|Local|GetVOIPIconVisible?))
    (Variables|Traitement|Local|SetVOIPIconVisible? Visible?)
    (bind _charref (Utilities|GetCharRef)
      (:Is%20Valid
        (bind _widgetvoiceref (Class|BPVOIPInterface|MSGAVPGetWidgetVoice(Message) _charref))
        (Rendering|SetVisibility _widgetvoiceref (Variables|Traitement|Local|GetVOIPIconVisible?) true)))))

(event Custom|CallSetAttenuationOnTeam
  (params (PassToAnotherPlayer? :type Boolean) (InSameTeam? :type Boolean) (ToPlayerRef :type Character%20Object%20Reference) (FromPlayerRef :type Character%20Object%20Reference))
  ;[1 1 1] Call RefreshAttenuationOnTeam on client (OnTeam)
  (if PassToAnotherPlayer?
    (CallFunction|ServerSendSetAttenuationonTeam InSameTeam? ToPlayerRef FromPlayerRef)
    (else
      (CallFunction|ClientRefreshAttenuationonTeam InSameTeam? FromPlayerRef))))

(event Custom|Local_SetIsMuted
  (params (Mute? :type Boolean) (InMyTeam :type Boolean))
  (bind _myvoiceref (Variables|Default|GetMyVoiceRef))
  ;[1 1 1] (Locally) Mute/Unmute the player
  (bind _output_get (Variables|Traitement|Local|SetIsMuted? Mute?))
  (Utilities|IsValid _myvoiceref
    (:Is%20Valid
      (Utilities|Struct|SetmembersinVoiceSettings (Variables|/Script/Engine.VOIPTalker|GetSettings _myvoiceref) (Traitement|GetAttenutation InMyTeam _output_get)))))

(event Custom|Client_PlayBip
  (params (Sound :type Sound%20Cue%20Object%20Reference))
  (bind _characterref (Variables|Spawn|GetCharacterRef))
  ;[1 1 1] Play sound on player
  (Utilities|FlowControl|DoOnce false :!label _label
    (:Completed
      (Utilities|FlowControl|Sequence
        (:then_0
          (Utilities|GetIsLocallyControlled _characterref
            (:true
              (Audio|PlaySoundatLocation Sound (Transformation|GetActorLocation _characterref) "0, 0, 0" 1.0 1.0 0.0 0 0 0 0))))
        (:then_1
          (Utilities|FlowControl|Delay 0.3)
          (goto _label Reset))))))

(event EventBeginPlay
  (bind _attempt (Variables|Spawn|GetAttempt))
  ;[1 1 1] OnConstruct
  (Utilities|FlowControl|Delay 1.0)
  (CallFunction|CreateVOIP)
  (Development|ExecuteConsoleCommand (select (Variables|Settings|GetVOIPLoopBack?) "OSS.VoiceLoopback 1" "OSS.VoiceLoopback 0") 0)
  ;;[1 1 1] Get Controller (if player), security to prevent looping for uncontrolled
  (Utilities|GetIsLocallyControlled (Components|GetOwner) :!label _label
    (:false
      (if (<= _attempt 15)
        (Math|Integer|IncrementInt _attempt
          (:%20%20
            (Utilities|FlowControl|Delay 1.0)
            (goto _label)))))
    (:NotValid
      (Utilities|FlowControl|Delay 0.2)
      (goto _label))))

(fn GetAttenutation
  (params (InMyTeam :type Boolean) (IsMuted? :type Boolean))
  (return (select IsMuted? "/Game/AntizeVOIPSystem/Audio/SA_VOIPAttenuationMute.SA_VOIPAttenuationMute" (select InMyTeam "/Game/AntizeVOIPSystem/Audio/SA_VOIPAttenuationTeam.SA_VOIPAttenuationTeam" "/Game/AntizeVOIPSystem/Audio/SA_VOIPAttenuation.SA_VOIPAttenuation"))))

(fn GetIsinSameTeam
  (params (TeamID_1 :type Integer) (TeamID_2 :type Integer))
  (if (>= TeamID_2 0)
    (return (== TeamID_1 TeamID_2))
    (else
      (return false))))

(fn CanPassonTeam
  (params (PlayerTeamID :type Integer) (MyTeamNewID :type Integer) (MyTeamOldID :type Integer))
  (if (>= PlayerTeamID 0)
    (return (or (== PlayerTeamID MyTeamNewID) (== PlayerTeamID MyTeamOldID)))
    (else
      (return false))))

(fn CheckforVOIP
  (bind _hudref (Variables|Spawn|GetHUDRef))
  (bind _hudref_2 (Variables|Spawn|GetHUDRef))
  (bind _outactors (Actor|GetAllActorswithInterface "/Game/AntizeVOIPSystem/Blueprints/BP_VOIPInterface.BP_VOIPInterface_C"))
  (for _array_element _outactors
    (bind _output_get (LocalVariables|SetLocal_ArrayActorRef _array_element))
    (Utilities|IsValid _output_get
      (:Is%20Valid
        (bind _reference (Utilities|GetComponentbyActorRef (LocalVariables|GetLocal_ArrayActorRef))
          (:IsValid
            (if (Variables|BP_AntizeVOIPComponent_C|GetIsVOIPActivated? _reference)
              (LocalVariables|SetLocal_IsMuted? (Variables|BP_AntizeVOIPComponent_C|GetIsMuted? _reference))
              (LocalVariables|SetLocal_IsTeam? (Traitement|GetIsinSameTeam (Variables|BP_AntizeVOIPComponent_C|GetTeamID _reference) (Variables|Traitement|GetTeamID)))
              (LocalVariables|SetLocal_IsVisible? (<= (Math|Vector|VectorLength (- (Transformation|GetActorLocation (LocalVariables|GetLocal_ArrayActorRef)) (Transformation|GetActorLocation (Variables|Spawn|GetCharacterRef)))) (select (LocalVariables|GetLocal_IsTeam?) (Variables|Settings|GetMaxDistanceForTeamVOIPWidget) (Variables|Settings|GetMaxDistanceForVOIPWidget))))
              (Utilities|FlowControl|Sequence
                (:then_0
                  (if (LocalVariables|GetLocal_IsVisible?)
                    (Utilities|IsValid _hudref
                      (:Is%20Valid
                        (Default|RefreshVOIPList _hudref true (LocalVariables|GetLocal_ArrayActorRef)))
                      (:Is%20Not%20Valid
                        _))
                    (if (!= (LocalVariables|GetLocal_ArrayActorRef) (Variables|Spawn|GetCharacterRef))
                      (bind (_outhit _returnvalue) (Collision|LineTraceByChannel (Transformation|GetActorLocation (Variables|Spawn|GetCharacterRef)) (Transformation|GetActorLocation (LocalVariables|GetLocal_ArrayActorRef)) "TraceTypeQuery1" false (Utilities|Array|MakeArray (Variables|Spawn|GetCharacterRef)) "None"))
                      (if _returnvalue
                        (Traitement|SetVisibilityVOIPIconbyActorRef (LocalVariables|GetLocal_ArrayActorRef) (== (LocalVariables|GetLocal_ArrayActorRef) (.HitActor (Collision|BreakHitResult _outhit))))
                        (else
                          (Traitement|SetVisibilityVOIPIconbyActorRef (LocalVariables|GetLocal_ArrayActorRef) false))))
                    (else
                      (Utilities|IsValid _hudref_2 :!label _label
                        (:Is%20Valid
                          (Default|RefreshVOIPList _hudref_2 false (LocalVariables|GetLocal_ArrayActorRef)))
                        (:Is%20Not%20Valid
                          _))
                      (Traitement|SetVisibilityVOIPIconbyActorRef (LocalVariables|GetLocal_ArrayActorRef) false))))
                (:then_1
                  ;[1 1 1] For sound effect
                  (if (!= (Variables|Spawn|GetCharacterRef) (LocalVariables|GetLocal_ArrayActorRef))
                    (if (not (LocalVariables|GetLocal_IsMuted?))
                      (Utilities|FlowControl|DoOnce false :!label _label_2
                        (:Completed
                          (if (or (LocalVariables|GetLocal_IsVisible?) (LocalVariables|GetLocal_IsTeam?))
                            (LocalVariables|SetLocal_HasTalker? true)
                            (else
                              (goto _label_2 Reset)))))))))
              (else
                (goto _label))))
          (:IsNotValid
            (goto _label))))))
  (Traitement|Sound|OnEffectSound (LocalVariables|GetLocal_HasTalker?))
  (return))

(fn SetVisibilityVOIPIconbyActorRef
  (params (ActorRef :type Actor%20Object%20Reference) (Visible? :type Boolean))
  (bind _reference (Utilities|GetComponentbyActorRef ActorRef)
    (:IsValid
      (CallFunction|LocalSetVisibilityVOIPIcon _reference Visible?)
      (return))
    (:IsNotValid
      (return))))

(fn OnJoinTeam
  (params (NewTeamID :type Integer))
  (LocalVariables|SetLocal_NewTeamID NewTeamID)
  (LocalVariables|SetLocal_OldTeamID (Variables|Traitement|GetTeamID))
  (if (!= (LocalVariables|GetLocal_NewTeamID) (Variables|Traitement|GetTeamID))
    (CallFunction|ServerSetTeamID (LocalVariables|GetLocal_NewTeamID))
    (Utilities|GetCharRef
      (:Is%20Valid
        (bind _outactors (Actor|GetAllActorswithInterface "/Game/AntizeVOIPSystem/Blueprints/BP_VOIPInterface.BP_VOIPInterface_C"))
        (for _array_element _outactors
          (Utilities|IsValid _array_element
            (:Is%20Valid
              (bind _ascharacter (Utilities|Casting|CastToCharacter _array_element))
              (bind _output_get (LocalVariables|SetLocal_ArrayCharRef _ascharacter))
              (if (!= _output_get (Variables|Spawn|GetCharacterRef))
                (bind _reference (Utilities|GetComponentbyActorRef (LocalVariables|GetLocal_ArrayCharRef))
                  (:IsValid
                    (if (Traitement|CanPassonTeam (Variables|BP_AntizeVOIPComponent_C|GetTeamID _reference) (LocalVariables|GetLocal_NewTeamID) (LocalVariables|GetLocal_OldTeamID))
                      (CallFunction|LocalRefreshAttenuationonTeam _reference (Traitement|GetIsinSameTeam (Variables|BP_AntizeVOIPComponent_C|GetTeamID _reference) (LocalVariables|GetLocal_NewTeamID)))
                      (CallFunction|CallSetAttenuationonTeam true (Traitement|GetIsinSameTeam (Variables|BP_AntizeVOIPComponent_C|GetTeamID _reference) (LocalVariables|GetLocal_NewTeamID)) (LocalVariables|GetLocal_ArrayCharRef) (Variables|Spawn|GetCharacterRef))))))))))
      (:NotValid
        _)))
  (return))

(fn ShowHidePlayerList
  (bind _playerlisrref (Variables|Spawn|GetPlayerLisrRef))
  (Utilities|IsValid _playerlisrref
    (:Is%20Valid
      (Default|ShowHide _playerlisrref false)
      (return))
    (:Is%20Not%20Valid
      (return))))

(fn OnRepTeamID
  (if (Variables|Traitement|GetPassOnRepTeamID)
    (CallFunction|CallonRepTeamID))
  (return))

(fn OnEffectSound
  (params (InHasTalker? :type Boolean))
  (if (Variables|Settings|GetPlayEffect?)
    (if (Math|Boolean|NotEqual(Boolean) InHasTalker? (Variables|Traitement|Sound|GetHasTalker?))
      (bind _output_get (Variables|Traitement|Sound|SetHasTalker? InHasTalker?))
      (if _output_get
        ;[1 1 1] Play or create a new sound effect
        (Utilities|IsValid (Variables|Traitement|Sound|GetSoundEffect)
          (:Is%20Valid
            (Class|AudioComponent|SetPaused (Variables|Traitement|Sound|GetSoundEffect) false))
          (:Is%20Not%20Valid
            (bind _returnvalue (Audio|SpawnSoundAttached "/Game/AntizeVOIPSystem/Audio/Cue_Effect.Cue_Effect" (Variables|/Script/Engine.Character|GetCapsuleComponent (Variables|Spawn|GetCharacterRef)) "None" "0, 0, 0" "0, 0, 0" "KeepRelativeOffset" true 1.0 1.0 0.0 0 0 false))
            (Variables|Traitement|Sound|SetSoundEffect _returnvalue)))
        (return)
        (else
          ;[1 1 1] Pause the sound effect if valid
          (Utilities|IsValid (Variables|Traitement|Sound|GetSoundEffect)
            (:Is%20Valid
              (Class|AudioComponent|SetPaused (Variables|Traitement|Sound|GetSoundEffect) true))
            (:Is%20Not%20Valid
              _))
          (return))))))

(fn OnBip
  (if (Variables|Settings|GetPlayEffect?)
    (Utilities|GetCharRef
      (:Is%20Valid
        (bind _outactors (Actor|GetAllActorswithInterface "/Game/AntizeVOIPSystem/Blueprints/BP_VOIPInterface.BP_VOIPInterface_C"))
        (for _array_element _outactors
          (bind _reference (Utilities|GetComponentbyActorRef _array_element)
            (:IsValid
              (if (Traitement|GetIsinSameTeam (Variables|BP_AntizeVOIPComponent_C|GetTeamID _reference) (Variables|Traitement|GetTeamID))
                (CallFunction|ServerPlayBiponPlayer _reference "/Game/AntizeVOIPSystem/Audio/Cue_Bip.Cue_Bip" :!label _label)
                (elif (<= (Math|Vector|VectorLength (- (Transformation|GetActorLocation _array_element) (Transformation|GetActorLocation (Variables|Spawn|GetCharacterRef)))) (Variables|Settings|GetMaxDistanceForVOIPWidget))
                  (goto _label)))))))
      (:NotValid
        _)))
  (return))

(fn FlipFlopSoundEffect
  (bind _soundeffect (Variables|Traitement|Sound|GetSoundEffect))
  (Variables|Settings|SetPlayEffect? (not (Variables|Settings|GetPlayEffect?)))
  (if (Variables|Traitement|Sound|GetHasTalker?)
    (Variables|Traitement|Sound|SetHasTalker? false)
    (Utilities|IsValid _soundeffect
      (:Is%20Valid
        (Class|AudioComponent|SetPaused _soundeffect true)))))